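; ROS 2 subscriber node Blueprint that listens for string messages on a test topic and prints them.
; On BeginPlay it initializes the node and adds a ROS2StringMsg subscription with a callback delegate made through a Create Event node.
; An event and a separate function hold identical callback logic, casting the incoming message to ROS2StringMsg and printing its string form.
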(event `self.ReceiveBeginPlay`
  (`self.Init`)
  (`self.AddSubscription` "test_topic" "/Script/rclUE.ROS2StringMsg" (`|CreateDelegate` :!event `ROS2Subscriber CB`)))

(event `SubscriptionCallback`
  (params (Message :type "ROS2GenericMsg Object Reference"))
  (`KismetSystemLibrary.PrintString` (`ROS2GenericMsg.MsgToString` (cast `ROS2StringMsg` Message :!pure true))))

(fn `ROS2Subscriber CB`
  (params (Message :type "ROS2GenericMsg Object Reference"))
  (`KismetSystemLibrary.PrintString` (`ROS2GenericMsg.MsgToString` (cast `ROS2StringMsg` Message :!pure true))))

(fn `UserConstructionScript`)