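; Example ROS 2 node Blueprint that hosts an AddTwoInts service server inside Unreal.
; On BeginPlay it initializes its ROS2Node, binds ServiceCallback to the service server and registers that server with the node.
; The callback casts the incoming service to ROS2AddTwoIntsSrv, sets the response to the sum of request fields A and B, and prints the operands and result.
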(event `self.ReceiveBeginPlay`
  (bind _ros2node (`self.ROS2Node`))
  (bind _serviceserver (`ROS2ServiceServerComponent.ServiceServer` (`self.ROS2ServiceServer`)))
  (`ROS2NodeComponent.Init` _ros2node)
  (`ROS2ServiceServer.SetDelegates` _serviceserver (delegate `ServiceCallback`))
  (`ROS2NodeComponent.AddServiceServer` _ros2node _serviceserver))

(event `ServiceCallback`
  (params (InService :type "ROS2GenericSrv Object Reference"))
  (bind _asros2add_two_ints_srv (cast `ROS2AddTwoIntsSrv` InService :!pure true))
  (bind (_request_a _request_b) (break `ROSAddTwoIntsReq` (`ROS2AddTwoIntsSrv.GetRequest` _asros2add_two_ints_srv)))
  (bind _returnvalue (+ _request_a _request_b))
  (`ROS2AddTwoIntsSrv.SetResponse` _asros2add_two_ints_srv (make `ROSAddTwoIntsRes` _returnvalue))
  (`KismetSystemLibrary.PrintString` (`KismetStringLibrary.Concat_StrStr` "add two ints server call back in BP " (`KismetStringLibrary.Conv_IntToString` (`KismetMathLibrary.Conv_Int64ToInt` _request_a)) " + " (`KismetStringLibrary.Conv_IntToString` (`KismetMathLibrary.Conv_Int64ToInt` _request_b)) " = " (`KismetStringLibrary.Conv_IntToString` (`KismetMathLibrary.Conv_Int64ToInt` _returnvalue)))))

(fn `UserConstructionScript`)