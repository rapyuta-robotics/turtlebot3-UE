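; Example ROS 2 node Blueprint that acts as a service client for an AddTwoInts service.
; On BeginPlay it initializes the node, binds request and response delegates, registers the client and starts a looping timer that periodically sends a request.
; The request callback fills in A and B, prints them and increments both for the next call.
; The response callback prints the returned sum on screen.
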(event `self.ReceiveBeginPlay`
  (bind _ros2serviceclient (`self.ROS2ServiceClient`))
  (`self.Init`)
  (set `ROS2ServiceClient.ResponseDelegate` (`|CreateDelegate` :!event `ROS2Request_Update`) _ros2serviceclient)
  (set `ROS2ServiceClient.RequestDelegate` (`|CreateDelegate` :!event `ROS2Response_Callback`) _ros2serviceclient)
  (`self.AddServiceClient` _ros2serviceclient)
  (`ROS2ServiceClient.Init` _ros2serviceclient "DynamicBroadcaster")
  (`KismetSystemLibrary.K2_SetTimerDelegate` (delegate `SrvCall`) 1.0 true))

(event `SrvCall`
  (`ROS2ServiceClient.UpdateAndSendRequest` (`self.ROS2ServiceClient`)))

(fn `ROS2Request_Update`
  (params (InService :type "ROS2GenericSrv Object Reference"))
  (bind _a (`self.A`))
  (bind _b (`self.B`))
  (`ROS2AddTwoIntsSrv.SetRequest` (cast `ROS2AddTwoIntsSrv` InService :!pure true) (make `ROSAddTwoInts_Request` (`KismetMathLibrary.Conv_IntToInt64` _a) (`KismetMathLibrary.Conv_IntToInt64` _b)))
  (`KismetSystemLibrary.PrintString` (`KismetStringLibrary.Concat_StrStr` "add two ints client send request in BP. " "a:" (`KismetStringLibrary.Conv_IntToString` _a) ", b:" (`KismetStringLibrary.Conv_IntToString` _b)))
  (set `self.A` (+ (`self.A`) 1))
  (set `self.B` (+ (`self.B`) 1)))

(fn `ROS2Response_Callback`
  (params (InService :type "ROS2GenericSrv Object Reference"))
  (bind _response_sum (break `ROSAddTwoInts_Response` (`ROS2AddTwoIntsSrv.GetResponse` (cast `ROS2AddTwoIntsSrv` InService :!pure true))))
  (`KismetSystemLibrary.PrintString` (`KismetStringLibrary.Concat_StrStr` "add two ints client receive request in BP. sum:" (`KismetStringLibrary.Conv_IntToString` (`KismetMathLibrary.Conv_Int64ToInt` _response_sum)))))

(fn `UserConstructionScript`)