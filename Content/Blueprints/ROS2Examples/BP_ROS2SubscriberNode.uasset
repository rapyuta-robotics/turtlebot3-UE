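; Example ROS 2 subscriber Blueprint that receives string messages on a topic and prints them.
; On BeginPlay it initializes its ROS2Node, binds CallbackEvent to ROS2Subscriber as a delegate and adds the subscription to the node.
; The callback casts each message to ROS2StrMsg and prints its data.
; A separate ROS2SubscriberCB function duplicates that print logic but is not bound in the event graph.
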(event `self.ReceiveBeginPlay`
  (bind _ros2node (`self.ROS2Node`))
  (bind _ros2subscriber (`self.ROS2Subscriber`))
  (`ROS2NodeComponent.Init` _ros2node)
  (`ROS2Subscriber.SetDelegates` _ros2subscriber (delegate `CallbackEvent`))
  (`ROS2NodeComponent.AddSubscription` _ros2node _ros2subscriber))

(event `CallbackEvent`
  (params (InMessage :type "ROS2GenericMsg Object Reference"))
  (bind _output_data (break `ROSStr` (`ROS2StrMsg.GetMsg` (cast `ROS2StrMsg` InMessage :!pure true))))
  ;[1 1 1] Topic subscription callback
  (`KismetSystemLibrary.PrintString` _output_data))

(fn `ROS2Subscriber CB`
  (params (Message :type "ROS2GenericMsg Object Reference"))
  (bind _output_data (break `ROSStr` (`ROS2StrMsg.GetMsg` (cast `ROS2StrMsg` Message :!pure true))))
  (`KismetSystemLibrary.PrintString` _output_data))

(fn `UserConstructionScript`)