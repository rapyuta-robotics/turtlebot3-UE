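; Example ROS 2 node Blueprint that acts as a Fibonacci action client.
; On BeginPlay it initializes, registers the client with its delegates, and retries sending the goal every second until the send succeeds.
; An accepted goal requests the result and increments the order; each result sends the next goal, forming a loop.
; Callbacks print progress; cancel is empty, and rejection only logs despite its "send goal again" message.
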(event `self.ReceiveBeginPlay`
  (bind _ros2actionclient (`self.ROS2ActionClient`))
  (`self.Init`)
  (`ROS2ActionClient.SetDelegates` (`self.ROS2ActionClient`) (`|CreateDelegate` :!event `SendGoal`) (`|CreateDelegate` :!event `FeedbackCallback`) (`|CreateDelegate` :!event `ResultCallback`) (`|CreateDelegate` :!event `Goal Response Callback`) (delegate `CancelDelegate`))
  (`self.AddActionClient` _ros2actionclient)
  (bind _returnvalue (`ROS2ActionClient.UpdateAndSendGoal` _ros2actionclient :!label _label))
  (if (not _returnvalue)
    (`KismetSystemLibrary.Delay` 1.0)
    (goto _label)))

(event `CancelDelegate`)

(fn `FeedbackCallback`
  (params (InAction :type "ROS2GenericAction Object Reference"))
  (bind _feedback_sequence (break `ROSFibonacci_FeedbackMessage` (`ROS2FibonacciAction.GetFeedback` (cast `ROS2FibonacciAction` InAction :!pure true))))
  (`KismetSystemLibrary.PrintString` (`KismetStringLibrary.Concat_StrStr` "[BP][fibonacci action] received feedback. last element is  " (`KismetStringLibrary.Conv_IntToString` (`|GetArrayItem` _feedback_sequence (`KismetArrayLibrary.Array_LastIndex` _feedback_sequence))))))

(fn `Goal Response Callback`
  (params (InAction :type "ROS2GenericAction Object Reference"))
  (bind _goal_accepted (break `ROSFibonacci_SendGoal_Response` (`ROS2FibonacciAction.GetGoalResponse` (cast `ROS2FibonacciAction` InAction :!pure true))))
  (if _goal_accepted
    (`ROS2ActionClient.GetResultRequest` (`self.ROS2ActionClient`))
    (`/Engine/EditorBlueprintResources/StandardMacros.IncrementInt` (`self.Order`)
      (:`  `
        (`KismetSystemLibrary.PrintString` "[BP][fibonacci action] received goal response. goal is accepted.")))
    (else
      (`KismetSystemLibrary.PrintString` "[BP][fibonacci action] received goal response. goal is rejected. send goal again."))))

(fn `ResultCallback`
  (params (InAction :type "ROS2GenericAction Object Reference"))
  (locals (NewLocalVar_0 :type Integer :default 0) (NewLocalVar_1 :type "Array of Integer"))
  (bind _result_sequence (break `ROSFibonacci_GetResult_Response` (`ROS2FibonacciAction.GetResultResponse` (cast `ROS2FibonacciAction` InAction :!pure true))))
  (set `self.ResultString` "")
  (bind _output_get (set `local.NewLocalVar_1` _result_sequence))
  (for _array_element _output_get
    (set `self.ResultString` (`KismetStringLibrary.Concat_StrStr` (`self.ResultString`) (`KismetStringLibrary.Conv_IntToString` _array_element) ", ")))
  (`KismetSystemLibrary.PrintString` (`KismetStringLibrary.Concat_StrStr` "[BP][fibonacci action] received result: " (`self.ResultString`)))
  (`ROS2ActionClient.UpdateAndSendGoal` (`self.ROS2ActionClient`)))

(fn `SendGoal`
  (params (InAction :type "ROS2GenericAction Object Reference"))
  (locals (GoalRequest :type "ROSFibonacci_SendGoal_Request Structure"))
  (bind _order (`self.Order`))
  (`ROS2FibonacciAction.SetGoalRequest` (cast `ROS2FibonacciAction` InAction :!pure true) (make `ROSFibonacci_SendGoal_Request` _order))
  (`KismetSystemLibrary.PrintString` (`KismetStringLibrary.Concat_StrStr` "[BP][fibonacci action] send goal, order: " (`KismetStringLibrary.Conv_IntToString` _order))))

(fn `UserConstructionScript`)