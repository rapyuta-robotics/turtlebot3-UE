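; Example ROS 2 action server actor that serves a Fibonacci action.
; BeginPlay initializes the ROS2Node and registers the server with goal, cancel and result delegates.
; Goals are always accepted; the result callback seeds the sequence and starts a looping timer that calls Execute to append a term and send feedback.
; Reaching the requested order sends the result and clears the timer, while cancel clears it and responds.
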(event `self.ReceiveBeginPlay`
  (bind _ros2node (`self.ROS2Node`))
  (bind _ros2actionserver (`self.ROS2ActionServer`))
  (`ROS2NodeComponent.Init` _ros2node)
  (`ROS2ActionServer.SetDelegates` _ros2actionserver (delegate `GoalCallback`) (delegate `CancelCallback`) (delegate `ResultCallback`))
  (`ROS2NodeComponent.AddActionServer` _ros2node _ros2actionserver))

(event `GoalCallback`
  (params (InAction :type "ROS2GenericAction Object Reference"))
  (bind _ros2actionserver (`self.ROS2ActionServer`))
  (bind _output_get (set `self.Goal` (`ROS2FibonacciAction.GetGoalRequest` (cast `ROS2FibonacciAction` InAction :!pure true))))
  (`ROS2FibonacciAction.SetGoalResponse` (cast `ROS2FibonacciAction` (`ROS2Action.Action` _ros2actionserver) :!pure true) (make `ROSFibonacciSGRes` true (`GameplayStatics.GetTimeSeconds`)))
  (`ROS2ActionServer.SendGoalResponse` _ros2actionserver)
  (`KismetSystemLibrary.PrintString` (`KismetStringLibrary.Concat_StrStr` "[BP][fibonacci action][goal callback] received goal. order: " (`KismetStringLibrary.Conv_IntToString` (break `ROSFibonacciSGReq` _output_get)))))

(event `CancelCallback`
  (`KismetSystemLibrary.K2_ClearAndInvalidateTimerHandle` (`self.ActionTimerHandle`))
  (`ROS2ActionServer.ProcessAndSendCancelResponse` (`self.ROS2ActionServer`) 0)
  (`KismetSystemLibrary.PrintString` "[BP][fibonacci action][cancel callback] received cancel request"))

(event `ResultCallback`
  (bind _fb_sequence (break `ROSFibonacciFB` (`self.FB`)))
  (`KismetArrayLibrary.Array_Clear` _fb_sequence)
  (`KismetArrayLibrary.Array_Add` _fb_sequence)
  (`KismetArrayLibrary.Array_Add` _fb_sequence 1)
  (`KismetSystemLibrary.PrintString` "[BP][fibonacci action][accepted delegate]  Start fibonacci calculation")
  (bind _returnvalue (`KismetSystemLibrary.K2_SetTimerDelegate` (delegate `CustomEvent`) 1.0 true))
  (set `self.ActionTimerHandle` _returnvalue))

(event `CustomEvent`
  (`self.Execute`))

(fn `Execute`
  (bind _fb_sequence (break `ROSFibonacciFB` (`self.FB`)))
  (bind _fb_sequence_2 (break `ROSFibonacciFB` (`self.FB`)))
  (bind _fb_sequence_3 (break `ROSFibonacciFB` (`self.FB`)))
  (bind _goal_order (break `ROSFibonacciSGReq` (`self.Goal`)))
  (bind _fb_sequence_4 (break `ROSFibonacciFB` (`self.FB`)))
  (bind _ros2actionserver (`self.ROS2ActionServer`))
  (bind _returnvalue (`KismetArrayLibrary.Array_LastIndex` _fb_sequence_4))
  (`KismetArrayLibrary.Array_Add` _fb_sequence_4 (+ (`|GetArrayItem` _fb_sequence_4 _returnvalue) (`|GetArrayItem` _fb_sequence_4 (- _returnvalue 1))))
  (if (>= (`KismetArrayLibrary.Array_Length` _fb_sequence_4) _goal_order)
    (`ROS2FibonacciAction.SetResultResponse` (cast `ROS2FibonacciAction` (`ROS2Action.Action` _ros2actionserver) :!pure true) (make `ROSFibonacciGRRes` _fb_sequence_2))
    (`ROS2ActionServer.SendResultResponse` _ros2actionserver)
    (`KismetSystemLibrary.K2_ClearAndInvalidateTimerHandle` (`self.ActionTimerHandle`))
    (set `self.ResultString` "")
    (for _array_element _fb_sequence
      (set `self.ResultString` (`KismetStringLibrary.Concat_StrStr` (`self.ResultString`) (`KismetStringLibrary.Conv_IntToString` _array_element) ", ")))
    (`KismetSystemLibrary.PrintString` (`KismetStringLibrary.Concat_StrStr` "[BP][fibonacci action] Send result:    " (`self.ResultString`)))
    (else
      (`ROS2FibonacciAction.SetFeedback` (cast `ROS2FibonacciAction` (`ROS2Action.Action` (`self.ROS2ActionServer`)) :!pure true) (make `ROSFibonacciFB` _fb_sequence_3))
      (`ROS2ActionServer.SendFeedback` (`self.ROS2ActionServer`))
      (`KismetSystemLibrary.PrintString` (`KismetStringLibrary.Concat_StrStr` "[BP][fibonacci action] update feedback. added value is   " (`KismetStringLibrary.Conv_IntToString` (`|GetArrayItem` _fb_sequence_3 (`KismetArrayLibrary.Array_LastIndex` _fb_sequence_3))))))))

(fn `UserConstructionScript`)