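; Example Blueprint that sets up a ROS2 node on BeginPlay and demonstrates three ways of publishing messages from Blueprint.
; A non-loop publisher sends a single string message after a short delay.
; A loop publisher uses a delegate, TimerEvent, to fill each string message with an incrementing count.
; A custom string publisher class is also added to the node, with no message logic in this graph.
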(event `self.ReceiveBeginPlay`
  (bind _looppublisher (`self.LoopPublisher`))
  (bind _nonlooppublisher (`self.NonLoopPublisher`))
  (`|ExecutionSequence`
    (:`then_0`
      (`ROS2NodeComponent.Init` (`self.ROS2Node`))
      ;[1 1 1] Non Loop Publisher
      (`ROS2NodeComponent.AddPublisher` (`self.ROS2Node`) _nonlooppublisher)
      (`KismetSystemLibrary.Delay` 3.0)
      ;;[1 1 1] Set Msg and Publish
      (`ROS2StrMsg.SetMsg` (cast `ROS2StrMsg` (`ROS2Topic.TopicMessage` _nonlooppublisher) :!pure true) (make `ROSStr` "Hello from BP fron non loop publisher"))
      (`ROS2Publisher.Publish` _nonlooppublisher))
    (:`then_1`
      ;[1 1 1] Loop Publisher
      (`ROS2Publisher.SetDelegates` _looppublisher (delegate `TimerEvent`))
      (`ROS2NodeComponent.AddPublisher` (`self.ROS2Node`) _looppublisher))
    (:`then_2`
      ;[1 1 1] Custom Publisher Class
      (`ROS2NodeComponent.AddPublisher` (`self.ROS2Node`) (`self.RRROS2StringPublisher`)))))

(event `TimerEvent`
  (params (InTopicMessage :type "ROS2GenericMsg Object Reference"))
  (bind _count (`self.Count`))
  ;[1 1 1] Loop Publisher
  (`ROS2StrMsg.SetMsg` (cast `ROS2StrMsg` InTopicMessage :!pure true) (make `ROSStr` (`KismetStringLibrary.Concat_StrStr` "Hello from BP " (`KismetStringLibrary.Conv_IntToString` _count))))
  (`/Engine/EditorBlueprintResources/StandardMacros.IncrementInt` _count))

(fn `UserConstructionScript`)