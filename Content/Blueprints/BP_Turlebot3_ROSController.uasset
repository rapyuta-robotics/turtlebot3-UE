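; AI controller that connects a possessed TurtleBot3 Waffle vehicle pawn to ROS 2.
; On possession it initializes a child-actor ROS 2 node in the vehicle's namespace, starts the lidar, and sets up static and odometry TF publishers.
; A cmd_vel subscription converts Twist messages into the movement component's linear and angular velocity.
; An odometry publisher callback converts the component's odometry to ROS coordinates and refreshes the odom TF.
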(event `self.ReceivePossess`
  (params (PossessedPawn :type "Pawn Object Reference"))
  (bind _base2lidartfpublisher (`self.Base2LidarTFPublisher`))
  (bind _odompublisher (`self.OdomPublisher`))
  (bind _asros2node (cast `ROS2Node` (`ChildActorComponent.ChildActor` (`self.ROS2Node`)) :!pure true))
  (bind _asbp_turtlebot_3_waffle_vehicle (cast `/Game/Blueprints/BP_Turtlebot3_Waffle_Vehicle` PossessedPawn))
  (`|ExecutionSequence`
    (:`then_0`
      ;[1 1 1] ROS Node Init, set namespace
      (set `ROS2Node.Namespace` (`/Game/Blueprints/BP_Turtlebot3_Waffle_Vehicle.namespace` _asbp_turtlebot_3_waffle_vehicle) _asros2node)
      (`ROS2Node.Init` _asros2node))
    (:`then_1`
      (bind _assensor_lidar (`self.GetLidar` _asbp_turtlebot_3_waffle_vehicle))
      ;[1 1 1] Lidar
      (`SensorLidar.InitToNode` _assensor_lidar _asros2node)
      (`SensorLidar.Run` _assensor_lidar))
    (:`then_2`
      ;[1 1 1] TF static
      (`TFPublisher.InitTfPublisher` _base2lidartfpublisher _asros2node)
      (set `TFPublisher.Tf` (`self.GetTransform` _assensor_lidar) _base2lidartfpublisher))
    (:`then_3`
      (`TFPublisher.InitTfPublisher` (`self.Footprint2LinkTFPublisher`) _asros2node))
    (:`then_4`
      ;[1 1 1] cmd_vel call back
      (`ROS2Node.AddSubscription` _asros2node "/cmd_vel" "/Script/rclUE.ROS2TwistMsg" (`|CreateDelegate` :!event `Cmd Vel Cb`)))
    (:`then_5`
      ;[1 1 1] Odom
      (set `ROS2Publisher.UpdateDelegate` (`|CreateDelegate` :!event `Odom Pub Update`) _odompublisher)
      (`ROS2Node.AddPublisher` _asros2node _odompublisher)
      (`ROS2Publisher.Init` _odompublisher "KeepLast")
      (`TFPublisher.InitTfPublisher` (`self.OdomTFPublisher`) _asros2node))))

(event `self.ReceiveBeginPlay`)

(fn `Cmd Vel Cb`
  (params (Message :type "ROS2GenericMsg Object Reference"))
  (bind _asros2twist_msg (cast `ROS2TwistMsg` Message :!pure true))
  (bind _movementcomponent (`/Game/Blueprints/BP_Turtlebot3_Waffle_Vehicle.MovementComponent` (cast `/Game/Blueprints/BP_Turtlebot3_Waffle_Vehicle` (`self.K2_GetPawn`) :!pure true)))
  (bind _returnvalue (`ROSUtility.VectorROSToUE` (`ROS2TwistMsg.GetLinearVelocity` _asros2twist_msg)))
  (set `MovementComponent.Velocity` _returnvalue _movementcomponent)
  (bind _returnvalue_2 (`ROSUtility.RotationROSToUE` (`ROS2TwistMsg.GetAngularVelocity` _asros2twist_msg)))
  (set `KinematicsMovementComponent.AngularVelocity` _returnvalue_2 _movementcomponent))

(fn `GetLidar`
  (params (self2 :type "/Game/Blueprints/BP_Turtlebot3_Waffle_Vehicle Object Reference"))
  (returns (`AsSensor Lidar` :type "SensorLidar Object Reference"))
  (return (cast `SensorLidar` (`ChildActorComponent.ChildActor` (`/Game/Blueprints/BP_Turtlebot3_Waffle_Vehicle.SensorLidar` self2)) :!pure true)))

(fn `Odom Pub Update`
  (params (TopicMessage :type "ROS2GenericMsg Object Reference"))
  (bind _movementcomponent (`/Game/Blueprints/BP_Turtlebot3_Waffle_Vehicle.MovementComponent` (cast `/Game/Blueprints/BP_Turtlebot3_Waffle_Vehicle` (`self.K2_GetPawn`) :!pure true)))
  (`|ExecutionSequence`
    (:`then_0`
      ;[1 1 1] OdomTopic
      (bind _returnvalue (`ROSUtility.OdomUEToROS` (`KinematicsMovementComponent.OdomData` _movementcomponent)))
      (`ROS2OdometryMsg.Update` (cast `ROS2OdometryMsg` TopicMessage :!pure true) _returnvalue))
    (:`then_1`
      ;[1 1 1] Odom TF update
      (bind _returnvalue_2 (`KinematicsMovementComponent.getOdomTf` _movementcomponent))
      (set `TFPublisher.Tf` _returnvalue_2 (`self.OdomTFPublisher`)))))

(fn `UserConstructionScript`)