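; Controller that bridges a possessed Turtlebot Waffle vehicle to ROS 2.
; On possess it initializes its ROS2Node child actor with the vehicle's namespace, starts the lidar on that node, sets up odometry and TF publishers, and prints attached actor names.
; Incoming cmd_vel twists are converted to Unreal coordinates and drive the movement component's linear and angular velocity.
; The odometry publisher's update callback converts that component's odometry to ROS and refreshes the TF.
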(event `self.ReceivePossess`
  (params (PossessedPawn :type "Pawn Object Reference"))
  (bind _asbp_turtlebot_3_waffle_vehicle (cast `/Game/Blueprints/kinematics/BP_TurtlebotWaffleVehicle` PossessedPawn :!pure true))
  (bind _odompublisher (`self.OdomPublisher`))
  (bind _assensor_lidar (`self.GetLidar` _asbp_turtlebot_3_waffle_vehicle))
  (bind _asros2node (cast `ROS2Node` (`ChildActorComponent.ChildActor` (`self.ROS2Node`)) :!pure true))
  (`|ExecutionSequence`
    (:`then_0`
      ;[1 1 1] ROS Node Init, set namespace
      (set `ROS2Node.Namespace` (`/Game/Blueprints/kinematics/BP_TurtlebotWaffleVehicle.namespace` _asbp_turtlebot_3_waffle_vehicle) _asros2node)
      (`ROS2Node.Init` _asros2node))
    (:`then_1`
      ;[1 1 1] Lidar
      (`SensorLidar.InitToNode` _assensor_lidar _asros2node)
      (`SensorLidar.Run` _assensor_lidar))
    (:`then_2`
      ;[1 1 1] Odom
      (set `ROS2Publisher.UpdateDelegate` (`|CreateDelegate` :!event `Odom Pub Update`) _odompublisher)
      (`ROS2Node.AddPublisher` _asros2node _odompublisher)
      (`ROS2Publisher.Init` _odompublisher "KeepLast")
      (`ROS2TFPublisher.InitTFPublisher` (`self.OdomTFPublisher`) _asros2node))
    (:`then_3`
      ;[1 1 1] cmd_vel call back
      (`ROS2Node.AddSubscription` _asros2node "/cmd_vel" "/Script/rclUE.ROS2TwistMsg" (`|CreateDelegate` :!event `Cmd Vel Cb`)))
    (:`then_4`
      (for _array_element (`self.GetAttachedActors` PossessedPawn true)
        (`KismetSystemLibrary.PrintString` (`KismetSystemLibrary.GetObjectName` _array_element) true true (struct :`G` 0.66 :`B` 1.0 :`A` 1.0) 100.0)))))

(event `self.ReceiveBeginPlay`)

(fn `Cmd Vel Cb`
  (params (Message :type "ROS2GenericMsg Object Reference"))
  (bind (_output_linear _output_angular) (break `ROSTwist` (`ROS2TwistMsg.GetMsg` (cast `ROS2TwistMsg` Message :!pure true))))
  (bind _robotvehiclemovement (`/Game/Blueprints/kinematics/BP_TurtlebotWaffleVehicle.RobotVehicleMovement` (cast `/Game/Blueprints/kinematics/BP_TurtlebotWaffleVehicle` (`self.K2_GetPawn`) :!pure true)))
  (bind _returnvalue (`ConversionUtils.VectorROSToUE` _output_linear))
  (set `MovementComponent.Velocity` _returnvalue _robotvehiclemovement)
  (bind _returnvalue_2 (`ConversionUtils.RotationROSToUE` _output_angular))
  (set `RobotVehicleMovementComponent.AngularVelocity` _returnvalue_2 _robotvehiclemovement))

(fn `GetLidar`
  (params (self2 :type "/Game/Blueprints/kinematics/BP_TurtlebotWaffleVehicle Object Reference"))
  (returns (`AsSensor Lidar` :type "SensorLidar Object Reference"))
  (return (cast `SensorLidar` (`ChildActorComponent.ChildActor` (`/Game/Blueprints/kinematics/BP_TurtlebotWaffleVehicle.SensorLidar` self2)) :!pure true)))

(fn `Odom Pub Update`
  (params (TopicMessage :type "ROS2GenericMsg Object Reference"))
  (bind _robotvehiclemovement (`/Game/Blueprints/kinematics/BP_TurtlebotWaffleVehicle.RobotVehicleMovement` (cast `/Game/Blueprints/kinematics/BP_TurtlebotWaffleVehicle` (`self.K2_GetPawn`) :!pure true)))
  (`|ExecutionSequence`
    (:`then_0`
      ;[1 1 1] OdomTopic
      (bind _returnvalue (`ConversionUtils.OdomUEToROS` (`RobotVehicleMovementComponent.OdomData` _robotvehiclemovement)))
      (`ROS2OdometryMsg.SetMsg` (cast `ROS2OdometryMsg` TopicMessage :!pure true) _returnvalue))
    (:`then_1`
      ;[1 1 1] Odom TF update
      (bind _returnvalue_2 (`RobotVehicleMovementComponent.GetOdomTF` _robotvehiclemovement))
      (set `ROS2TFPublisher.TF` _returnvalue_2 (`self.OdomTFPublisher`)))))

(fn `UserConstructionScript`)